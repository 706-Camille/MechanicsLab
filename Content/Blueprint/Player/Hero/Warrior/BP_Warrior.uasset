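; BP_Warrior is the player's Warrior hero character Blueprint, armed with a katana.
; On BeginPlay it snaps the Sword component to the S_KatanaR socket on the mesh.
; Left mouse and the 1 key are bound directly in the graph, asking the CombatComponent to activate abilities by gameplay tag for a light sword attack and the Spin Charge skill.
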(event `self.ReceiveBeginPlay`
  (`SceneComponent.K2_AttachToComponent` (`self.Sword`) (`self.Mesh`) "S_KatanaR" "SnapToTarget" "SnapToTarget" "SnapToTarget" true))

(event `Key|LeftMouseButton`
  (params (Key :type "Key Structure"))
  (:`Pressed`
    (`MLCombatComponent.TryActivateAbilityByTag` (`self.CombatComponent`) (`BlueprintGameplayTagLibrary.MakeLiteralGameplayTag` (struct :`TagName` "Player.Attack.Light.Sword")))))

(event `Key|One`
  (params (Key :type "Key Structure"))
  (:`Pressed`
    (`MLCombatComponent.TryActivateAbilityByTag` (`self.CombatComponent`) (`BlueprintGameplayTagLibrary.MakeLiteralGameplayTag` (struct :`TagName` "Player.Class.Warrior.Skill.SpinCharge")))))

(fn `UserConstructionScript`
  (`parent.UserConstructionScript`))