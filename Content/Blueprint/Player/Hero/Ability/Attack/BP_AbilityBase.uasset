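; BP_AbilityBase is a Gameplay Ability base for hero attacks, providing shared forward hit-detection helpers.
; Box and line trace functions sweep from the avatar's location along its forward vector for a given range, with box size set by the caller and orientation matching the avatar.
; Both return multiple hits on Pawn objects, ignore the avatar and draw timed debug shapes.
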(fn `ExecuteForwardBoxTrace`
  (params (`Trace Half Size` :type "Vector Structure") (TraceRange :type "Float (double-precision)"))
  (returns (OutHits :type "Array of HitResult Structure"))
  (locals (TraceHalfSize :type "Vector Structure" :default (0.0 0.0 0.0)))
  (bind (_owneractor _avataractor) (break `AbilityActorInfo` (`self.ActorInfo`)))
  (bind _returnvalue (`Actor.K2_GetActorRotation` _avataractor))
  (bind _returnvalue_2 (`Actor.K2_GetActorLocation` _avataractor))
  (bind _outhits (`KismetSystemLibrary.BoxTraceMultiForObjects` _returnvalue_2 (+ _returnvalue_2 (* (`KismetMathLibrary.Conv_RotatorToVector` _returnvalue) (`local.TraceRange`))) (`local.Trace Half Size`) _returnvalue (`|MakeArray` "ObjectTypeQuery3" :!type "EObjectTypeQuery Enum") false (`|MakeArray` _avataractor :!type "Actor Object Reference") "ForDuration"))
  (return _outhits))

(fn `ExecuteForwardLineTrace`
  (params (TraceRange :type "Float (double-precision)"))
  (returns (OutHits :type "Array of HitResult Structure"))
  (bind (_owneractor _avataractor) (break `AbilityActorInfo` (`self.ActorInfo`)))
  (bind _returnvalue (`Actor.K2_GetActorLocation` _avataractor))
  (bind _outhits (`KismetSystemLibrary.LineTraceMultiForObjects` _returnvalue (+ _returnvalue (* (`KismetMathLibrary.Conv_RotatorToVector` (`Actor.K2_GetActorRotation` _avataractor)) (`local.TraceRange`))) (`|MakeArray` "ObjectTypeQuery3" :!type "EObjectTypeQuery Enum") false (`|MakeArray` _avataractor :!type "Actor Object Reference") "ForDuration"))
  (return _outhits))